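; BP_Whitebot is the player character, with polled WASD movement, double jump, stamina-limited sprint, levitation, zoom and emotes.
; Alternating punch and kick montages use timers to sphere-trace and call ReceivePunch on BP_Enemy.
; Its own ReceivePunch reduces health and ragdolls it at zero, while engine damage events only print.
; Tick drives movement, levitation rise, camera FOV and distance, stamina, and camera-facing health and stamina bars built from scaled components.
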(event EventBeginPlay
  (bind _mesh (Variables|Character|GetMesh))
  ;[0.15 0.15 0.15 0.5] Comment
  (Components|SkinnedMesh|HideBonebyName _mesh "pistol" "PBO_None")
  (Components|SkinnedMesh|HideBonebyName _mesh "bazooka" "PBO_None")
  (Components|SkinnedMesh|HideBonebyName _mesh "boomerang" "PBO_None")
  (Components|SkinnedMesh|HideBonebyName _mesh "grenade" "PBO_None")
  (CallFunction|SetupStatsUI))

(event Collision|EventActorBeginOverlap
  (params (OtherActor :type Actor%20Object%20Reference)))

(event EventTick
  (params (DeltaSeconds :type Float%20%28single-precision%29))
  (CallFunction|HandleMovement)
  (CallFunction|LevitationTick)
  (CallFunction|UpdateFOV)
  (CallFunction|UpdateCameraDistance)
  (CallFunction|UpdateStamina)
  (CallFunction|UpdateStatsBars))

(event Game|Damage|EventAnyDamage
  (params (Damage :type Float%20%28single-precision%29) (DamageType :type Damage%20Type%20Object%20Reference) (InstigatedBy :type Controller%20Object%20Reference) (DamageCauser :type Actor%20Object%20Reference))
  (Development|PrintString (Utilities|String|Append "ANYDAMAGE Causer=" (Utilities|String|Append (Utilities|GetObjectName DamageCauser) (Utilities|String|Append "  DamageType=" (Utilities|GetClassDisplayName (Utilities|GetClass DamageType))))) true true "(R=0.000000,G=0.660000,B=1.000000,A=1.000000)" 2e+01))

(event Game|Damage|EventPointDamage
  (params (Damage :type Float%20%28single-precision%29) (DamageType :type Damage%20Type%20Object%20Reference) (HitLocation :type Vector :default "0, 0, 0") (HitNormal :type Vector :default "0, 0, 0") (HitComponent :type Primitive%20Component%20Object%20Reference) (BoneName :type Name :default "None") (ShotFromDirection :type Vector :default "0, 0, 0") (InstigatedBy :type Controller%20Object%20Reference) (DamageCauser :type Actor%20Object%20Reference) (HitInfo :type Hit%20Result%20Structure%20%28by%20ref%29))
  (Development|PrintString (Utilities|String|Append "POINTDAMAGE Causer=" (Utilities|String|Append (Utilities|GetObjectName DamageCauser) (Utilities|String|Append "  DamageType=" (Utilities|GetClassDisplayName (Utilities|GetClass DamageType))))) true true "(R=0.000000,G=0.660000,B=1.000000,A=1.000000)" 2e+01))

(event Input|MouseEvents|MouseX
  (params (AxisValue :type Float%20%28single-precision%29))
  (Pawn|Input|AddControllerYawInput AxisValue))

(event Input|MouseEvents|MouseY
  (params (AxisValue :type Float%20%28single-precision%29))
  (CallFunction|AddLookPitch AxisValue))

(event Input|MouseEvents|MouseWheelAxis
  (params (AxisValue :type Float%20%28single-precision%29))
  (CallFunction|ApplyZoom (* AxisValue -5e+01)))

(event Input|KeyboardEvents|T
  (params (Key :type Key%20Structure))
  (:Pressed
    (CallFunction|EmoteTalk)))

(event Input|KeyboardEvents|G
  (params (Key :type Key%20Structure))
  (:Pressed
    (CallFunction|EmoteKiss)))

(event Input|KeyboardEvents|H
  (params (Key :type Key%20Structure))
  (:Pressed
    (CallFunction|EmoteEat)))

(event Input|KeyboardEvents|SpaceBar
  (params (Key :type Key%20Structure))
  (:Pressed
    (CallFunction|HandleJump true))
  (:Released
    (CallFunction|HandleJump false)))

(event Input|MouseEvents|LeftMouseButton
  (params (Key :type Key%20Structure))
  (:Pressed
    (CallFunction|ExecutePunch)))

(event Input|KeyboardEvents|LeftAlt
  (params (Key :type Key%20Structure))
  (:Pressed
    (CallFunction|ToggleLevitation)))

(event Input|KeyboardEvents|LeftShift
  (params (Key :type Key%20Structure))
  (:Pressed
    (CallFunction|StartSprint))
  (:Released
    (CallFunction|StopSprint)))

(fn ConstructionScript)

(fn ReceivePunch
  (if (not (Variables|Default|GetbDead))
    (Variables|Default|SetHealth (- (Variables|Default|GetHealth) (Math|Float|MakeLiteralFloat 25.0)))
    (Development|PrintString "Damage Taken")
    (if (<= (- (Variables|Default|GetHealth) (Math|Float|MakeLiteralFloat 25.0)) (Math|Float|MakeLiteralFloat 0.0))
      (Variables|Default|SetbDead true)
      (Pawn|Components|CharacterMovement|DisableMovement (Variables|Character|GetCharacterMovement))
      (Collision|SetCollisionEnabled (Variables|Collision|GetCapsuleComponent) "NoCollision")
      (Collision|SetCollisionProfileName (Variables|Character|GetMesh) "Ragdoll" true :!class /Script/Engine.PrimitiveComponent)
      (Physics|SetSimulatePhysics (Variables|Character|GetMesh) true))))

(fn AddLookPitch
  (params (V :type Float%20%28double-precision%29))
  (Pawn|Input|AddControllerPitchInput self (- 0.0 V)))

(fn DoPunchHit
  (bind _returnvalue (Transformation|GetActorLocation))
  (bind _returnvalue_2 (Transformation|GetActorForwardVector))
  (bind (_outhit _returnvalue_3) (Collision|SphereTraceForObjects (+ _returnvalue (* _returnvalue_2 (Math|Float|MakeLiteralFloat 5e+01))) (+ _returnvalue (* _returnvalue_2 (Math|Float|MakeLiteralFloat 1.5e+02))) 45.0 (Utilities|Array|MakeArray (Utilities|Enum|LiteralenumEObjectTypeQuery "ObjectTypeQuery3")) false 0 "None"))
  (if _returnvalue_3
    (bind _asbp_enemy (Utilities|Casting|CastToBP_Enemy (.HitActor (Collision|BreakHitResult _outhit))))
    (Default|ReceivePunch _asbp_enemy)))

(fn EndPunch
  (Variables|Default|SetbPunching false))

(fn ToggleLevitation
  (if (not (Variables|Default|GetbDead))
    (if (Variables|Default|GetIsLevitating)
      (Variables|Default|SetIsLevitating false)
      (Components|Activation|Deactivate (Variables|Default|GetLevitationTrail))
      (Pawn|Components|CharacterMovement|SetMovementMode (Variables|Character|GetCharacterMovement) "MOVE_Falling" 0)
      (else
        (Variables|Default|SetIsLevitating true)
        (Variables|Default|SetLevitateStartZ (.Z (Math|Vector|BreakVector (Transformation|GetActorLocation))))
        (Components|Activation|Activate (Variables|Default|GetLevitationTrail) true)
        (Pawn|Components|CharacterMovement|SetMovementMode (Variables|Character|GetCharacterMovement) "MOVE_Flying" 0)))))

(fn LevitationTick
  (bind _returnvalue (Utilities|Time|GetWorldDeltaSeconds))
  (Variables|Default|SetLevitateInput (Math|Interpolation|FInterpTo (Variables|Default|GetLevitateInput) (select (and (Variables|Default|GetIsLevitating) (< (.Z (Math|Vector|BreakVector (Transformation|GetActorLocation))) (+ (Variables|Default|GetLevitateStartZ) (Math|Float|MakeLiteralFloat 45.0)))) (Math|Float|MakeLiteralFloat 1.0) (Math|Float|MakeLiteralFloat 0.0)) _returnvalue 4.0))
  (if (Variables|Default|GetIsLevitating)
    (Transformation|AddActorWorldOffset (Math|Vector|MakeVector 0.0 0.0 (* (* (Variables|Default|GetLevitateInput) (Math|Float|MakeLiteralFloat 1.5e+02)) _returnvalue)) true))
  (bind _asabp_unarmed (Utilities|Casting|CastToABP_Unarmed (Components|SkeletalMesh|GetAnimInstance (Variables|Character|GetMesh))))
  (Variables|/Game/Characters/Mannequins/Anims/Unarmed/ABP_Unarmed.ABP_Unarmed_C|SetIsLevitating _asabp_unarmed (Variables|Default|GetIsLevitating)))

(fn CheckDoubleJump
  (if (and (and (not (Variables|Default|GetbDead)) (not (Variables|Default|GetIsLevitating))) (and (AI|Components|NavMovement|IsFalling (Variables|Character|GetCharacterMovement)) (== (Variables|Default|GetJumpCurrentCount) (Class|KismetSystemLibrary|MakeLiteralInteger 1))))
    (Class|AnimInstance|PlaySlotAnimationasDynamicMontage (Components|SkeletalMesh|GetAnimInstance (Variables|Character|GetMesh)) "/Game/Characters/Mannequins/Anims/Unarmed/Jump/MM_Jump.MM_Jump" "DefaultSlot" 0.05 0.15 1.3 1 -1.0 0.0)))

(fn HandleMovement
  (bind _returnvalue (Game|GetPlayerController 0))
  (bind _returnvalue_2 (Pawn|GetController))
  (bind _self self)
  (bind _returnvalue_3 (Pawn|GetControlRotation _returnvalue_2 :!class /Script/Engine.Controller))
  (bind _yaw (Math|Rotator|BreakRotator _returnvalue_3))
  (bind _returnvalue_4 (Math|Rotator|MakeRotator 0.0 0.0 _yaw))
  (Variables|Default|SetMoveX (- (select (Game|Player|IsInputKeyDown _returnvalue "W") (Math|Float|MakeLiteralFloat 1.0) (Math|Float|MakeLiteralFloat 0.0)) (select (Game|Player|IsInputKeyDown _returnvalue "S") (Math|Float|MakeLiteralFloat 1.0) (Math|Float|MakeLiteralFloat 0.0))))
  (Variables|Default|SetMoveY (- (select (Game|Player|IsInputKeyDown _returnvalue "D") (Math|Float|MakeLiteralFloat 1.0) (Math|Float|MakeLiteralFloat 0.0)) (select (Game|Player|IsInputKeyDown _returnvalue "A") (Math|Float|MakeLiteralFloat 1.0) (Math|Float|MakeLiteralFloat 0.0))))
  (Utilities|IsValid _returnvalue_2
    (:Is%20Valid
      (Pawn|Input|AddMovementInput _self (Math|Vector|GetForwardVector _returnvalue_4) (Variables|Default|GetMoveX) false)
      (Pawn|Input|AddMovementInput _self (Math|Vector|GetRightVector _returnvalue_4) (Variables|Default|GetMoveY) false))))

(fn HandleJump
  (params (bPressed :type Boolean))
  (if bPressed
    (Character|Jump)
    (CallFunction|CheckDoubleJump)
    (else
      (Character|StopJumping))))

(fn ExecutePunch
  (bind _self self)
  (bind _mesh (Variables|Character|GetMesh))
  (bind _returnvalue (Components|SkeletalMesh|GetAnimInstance _mesh))
  (if (not (or (Variables|Default|GetbDead) (Variables|Default|GetbPunching)))
    (Variables|Default|SetbPunching true)
    (if (Variables|Default|GetbPunchRight)
      (Class|AnimInstance|PlaySlotAnimationasDynamicMontage _returnvalue "/Game/FreeAnimationsPack/Retargeted/AS_ComboHands_Drongo.AS_ComboHands_Drongo" "DefaultSlot" 0.1 0.2 1.4 1 -1.0 0.0)
      (else
        (Class|AnimInstance|PlaySlotAnimationasDynamicMontage _returnvalue "/Game/FreeAnimationsPack/Retargeted/AS_RightLegKick2_Drongo.AS_RightLegKick2_Drongo" "DefaultSlot" 0.1 0.2 1.4 1 -1.0 0.0)))
    (Variables|Default|SetbPunchRight (not (Variables|Default|GetbPunchRight)))
    (Utilities|Time|SetTimerbyFunctionName _self "DoPunchHit" 0.25)
    (Utilities|Time|SetTimerbyFunctionName _self "EndPunch" 0.6)))

(fn UpdateFOV
  (bind _camera (Variables|Default|GetCamera))
  (Camera|SetFieldOfView _camera (Math|Interpolation|FInterpTo (Variables|/Script/Engine.CameraComponent|GetFieldOfView _camera) (select (Variables|Default|GetIsLevitating) (Math|Float|MakeLiteralFloat 1.1e+02) (Math|Float|MakeLiteralFloat 9e+01)) (Utilities|Time|GetWorldDeltaSeconds) 6.0)))

(fn StartSprint
  (Variables|/Script/Engine.CharacterMovementComponent|SetMaxWalkSpeed (Variables|Character|GetCharacterMovement) 9.5e+02))

(fn StopSprint
  (Variables|/Script/Engine.CharacterMovementComponent|SetMaxWalkSpeed (Variables|Character|GetCharacterMovement) 6e+02))

(fn EmoteTalk
  (if (not (Variables|Default|GetbDead))
    (Class|AnimInstance|PlaySlotAnimationasDynamicMontage (Components|SkeletalMesh|GetAnimInstance (Variables|Character|GetMesh)) "/Game/FreeAnimationsPack/Retargeted/AS_Talk_Drongo.AS_Talk_Drongo" "UpperBody" 0.25 0.25 1.0 1 -1.0 0.0)))

(fn EmoteKiss
  (if (not (Variables|Default|GetbDead))
    (Class|AnimInstance|PlaySlotAnimationasDynamicMontage (Components|SkeletalMesh|GetAnimInstance (Variables|Character|GetMesh)) "/Game/FreeAnimationsPack/Retargeted/AS_AirKiss_Drongo.AS_AirKiss_Drongo" "UpperBody" 0.25 0.25 1.0 1 -1.0 0.0)))

(fn EmoteEat
  (if (not (Variables|Default|GetbDead))
    (Class|AnimInstance|PlaySlotAnimationasDynamicMontage (Components|SkeletalMesh|GetAnimInstance (Variables|Character|GetMesh)) "/Game/FreeAnimationsPack/Retargeted/AS_EatingOnParty_Drongo.AS_EatingOnParty_Drongo" "UpperBody" 0.25 0.25 1.0 1 -1.0 0.0)))

(fn UpdateCameraDistance
  (bind _springarm (Variables|Default|GetSpringArm))
  (Variables|/Script/Engine.SpringArmComponent|SetTargetArmLength _springarm (Math|Interpolation|FInterpTo (Variables|/Script/Engine.SpringArmComponent|GetTargetArmLength _springarm) (Math|Float|Clamp(Float) (+ (select (> (Math|Vector|VectorLengthXY (Transformation|GetVelocity)) (Math|Float|MakeLiteralFloat 3e+02)) (Math|Float|MakeLiteralFloat 5e+02) (Math|Float|MakeLiteralFloat 3e+02)) (Variables|Default|GetZoomOffset)) 1.5e+02 8e+02) (Utilities|Time|GetWorldDeltaSeconds) 4.0)))

(fn UpdateStamina
  (Variables|Default|SetStamina (Math|Float|Clamp(Float) (+ (Variables|Default|GetStamina) (* (select (and (> (Math|Vector|VectorLengthXY (Transformation|GetVelocity)) (Math|Float|MakeLiteralFloat 7.5e+02)) (not (Variables|Default|GetIsLevitating))) (Math|Float|MakeLiteralFloat -25.0) (Math|Float|MakeLiteralFloat 15.0)) (Utilities|Time|GetWorldDeltaSeconds))) 0.0 1e+02))
  (if (<= (Math|Float|Clamp(Float) (+ (Variables|Default|GetStamina) (* (select (and (> (Math|Vector|VectorLengthXY (Transformation|GetVelocity)) (Math|Float|MakeLiteralFloat 7.5e+02)) (not (Variables|Default|GetIsLevitating))) (Math|Float|MakeLiteralFloat -25.0) (Math|Float|MakeLiteralFloat 15.0)) (Utilities|Time|GetWorldDeltaSeconds))) 0.0 1e+02) (Math|Float|MakeLiteralFloat 0.0))
    (CallFunction|StopSprint)))

(fn UpdateStatsBars
  (bind _returnvalue (Math|Float|MakeLiteralFloat 1e+02))
  (bind _returnvalue_2 (Math|Float|MakeLiteralFloat 1e+02))
  (bind _health (Variables|Default|GetHealth))
  (bind _stamina (Variables|Default|GetStamina))
  (bind _returnvalue_3 (/ _health _returnvalue))
  (bind _returnvalue_4 (/ _stamina _returnvalue_2))
  (bind _returnvalue_5 (Math|Float|Clamp(Float) _returnvalue_3))
  (bind _returnvalue_6 (Math|Float|Clamp(Float) _returnvalue_4))
  (Transformation|SetWorldRotation (Variables|Default|GetUI_Stats) (Transformation|GetWorldRotation (Variables|Default|GetCamera)) false false)
  (Transformation|SetRelativeScale3D (Variables|Default|GetHealthBar) (Math|Vector|MakeVector 0.05 0.05 (* (Math|Float|MakeLiteralFloat 0.7) _returnvalue_5)))
  (Transformation|SetRelativeLocation (Variables|Default|GetHealthBar) (Math|Vector|MakeVector 0.0 (* (Math|Float|MakeLiteralFloat 35.0) (- _returnvalue_5 (Math|Float|MakeLiteralFloat 1.0))) 4.0) false false)
  (Transformation|SetRelativeScale3D (Variables|Default|GetStaminaBar) (Math|Vector|MakeVector 0.05 0.05 (* (Math|Float|MakeLiteralFloat 0.7) _returnvalue_6)))
  (Transformation|SetRelativeLocation (Variables|Default|GetStaminaBar) (Math|Vector|MakeVector 0.0 (* (Math|Float|MakeLiteralFloat 35.0) (- _returnvalue_6 (Math|Float|MakeLiteralFloat 1.0))) -4.0) false false))

(fn SetupStatsUI
  (Collision|SetCollisionEnabled (Variables|Default|GetHealthBack) "NoCollision")
  (Collision|SetCollisionEnabled (Variables|Default|GetHealthBar) "NoCollision")
  (Collision|SetCollisionEnabled (Variables|Default|GetStaminaBack) "NoCollision")
  (Collision|SetCollisionEnabled (Variables|Default|GetStaminaBar) "NoCollision"))

(fn ApplyZoom
  (params (Delta :type Float%20%28double-precision%29))
  (bind _springarm (Variables|Default|GetSpringArm))
  (Variables|/Script/Engine.SpringArmComponent|SetTargetArmLength _springarm (Math|Float|Clamp(Float) (+ (Variables|/Script/Engine.SpringArmComponent|GetTargetArmLength _springarm) Delta) 1.5e+02 8e+02))
  (Variables|Default|SetZoomOffset (Math|Float|Clamp(Float) (+ (Variables|Default|GetZoomOffset) Delta) -1.5e+02 3e+02)))