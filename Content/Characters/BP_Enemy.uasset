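; BP_Enemy is a melee enemy that chases player 0 from BeginPlay until it dies.
; An AI MoveTo loop retries until in range, then triggers a DoOnce-gated attack montage.
; After a short delay it calls ReceivePunch on a BP_Whitebot player still in range, then resumes chasing.
; Its own ReceivePunch subtracts fixed damage, re-subtracts it in the death check, and switches to ragdoll on death.
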(event Custom|ChasePlayer
  (bind _returnvalue (Game|GetPlayerCharacter 0))
  (if (not (Variables|Default|GetbDead))
    (AI|AIMoveTo self "0, 0, 0" _returnvalue 8e+01 false
      (:OnSuccess
        (if (<= (Transformation|GetDistanceTo _returnvalue 0) (Math|Float|MakeLiteralFloat 1.2e+02))
          (CallFunction|ExecuteAttack)
          (else
            (Utilities|FlowControl|Delay 0.2)
            (CallFunction|ChasePlayer))))
      (:OnFail
        (Utilities|FlowControl|Delay 0.2)
        (CallFunction|ChasePlayer)))))

(event Custom|ExecuteAttack
  (Utilities|FlowControl|DoOnce false :!label _label
    (:Completed
      (Class|NavMovementInterface|StopActiveMovement (Variables|Character|GetCharacterMovement))
      (Class|AnimInstance|PlaySlotAnimationasDynamicMontage (Components|SkeletalMesh|GetAnimInstance (Variables|Character|GetMesh)) "/Game/Characters/Mannequins/Anims/Unarmed/Attack/MM_Attack_01.MM_Attack_01" "DefaultSlot" 0.1 0.2 1.0 1 -1.0 0.0)
      (Utilities|FlowControl|Delay 0.4)
      (bind _asbp_whitebot (Utilities|Casting|CastToBP_Whitebot (Game|GetPlayerCharacter 0))
        (:then
          (if (<= (Transformation|GetDistanceTo _asbp_whitebot 0) (Math|Float|MakeLiteralFloat 1.3e+02))
            (Default|ReceivePunch _asbp_whitebot))
          (Utilities|FlowControl|Delay 1.5)
          (CallFunction|ChasePlayer)
          (goto _label Reset))
        (:CastFailed
          (Utilities|FlowControl|Delay 1.5)
          (CallFunction|ChasePlayer)
          (goto _label Reset))))))

(event EventBeginPlay
  (CallFunction|ChasePlayer))

(event Collision|EventActorBeginOverlap
  (params (OtherActor :type Actor%20Object%20Reference)))

(event EventTick
  (params (DeltaSeconds :type Float%20%28single-precision%29)))

(fn ConstructionScript)

(fn ReceivePunch
  (if (not (Variables|Default|GetbDead))
    (Variables|Default|SetHealth (- (Variables|Default|GetHealth) (Math|Float|MakeLiteralFloat 25.0)))
    (if (<= (- (Variables|Default|GetHealth) (Math|Float|MakeLiteralFloat 25.0)) (Math|Float|MakeLiteralFloat 0.0))
      (Variables|Default|SetbDead true)
      (Pawn|Components|CharacterMovement|DisableMovement (Variables|Character|GetCharacterMovement))
      (Collision|SetCollisionEnabled (Variables|Collision|GetCapsuleComponent) "NoCollision")
      (Collision|SetCollisionProfileName (Variables|Character|GetMesh) "Ragdoll" true :!class /Script/Engine.PrimitiveComponent)
      (Physics|SetSimulatePhysics (Variables|Character|GetMesh) true))))