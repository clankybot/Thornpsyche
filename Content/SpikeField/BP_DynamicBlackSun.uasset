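; BP_DynamicBlackSun is a SpikeField actor that spins continuously around the world yaw axis.
; Each Tick adds a world rotation from RotationSpeed and delta time, scaled down by a constant factor so it is frame-rate independent and slow.
; Two disconnected rotation variants, local pitch and unscaled world yaw, remain in the graph but never run.
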(event EventBeginPlay)

(event Collision|EventActorBeginOverlap
  (params (OtherActor :type Actor%20Object%20Reference)))

(event EventTick
  (params (DeltaSeconds :type Float%20%28single-precision%29))
  (Class|Actor|AddActorWorldRotation (Math|Rotator|MakeRotator 0.0 0.0 (* (Variables|Default|GetRotationSpeed) (* DeltaSeconds (Math|Float|MakeLiteralFloat 0.1))))))

(fn ConstructionScript)