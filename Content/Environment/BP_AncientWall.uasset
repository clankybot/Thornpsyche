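; Ancient wall actor that builds a broken square perimeter of wall segments around its origin.
; The Construction Script clears and refills the WallInstances instanced mesh component, laying twelve slots per side over four rotated sides.
; Modulo tests on the running segment index leave regular gaps and make some segments lower and narrower, giving a deterministic ruined look without randomness.
; The event graph holds no active logic.
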(event EventBeginPlay)

(event Collision|EventActorBeginOverlap
  (params (OtherActor :type Actor%20Object%20Reference)))

(event EventTick
  (params (DeltaSeconds :type Float%20%28single-precision%29)))

(fn ConstructionScript
  (bind _wallinstances (Variables|Default|GetWallInstances))
  (Components|InstancedStaticMesh|ClearInstances _wallinstances)
  (for _index (range 0 3)
    (for _index_2 (range 0 11)
      (if (not (== (Math|Integer|%(Integer) (+ (* _index (Class|KismetSystemLibrary|MakeLiteralInteger 12)) _index_2) 5) (Class|KismetSystemLibrary|MakeLiteralInteger 3)))
        (Components|InstancedStaticMesh|AddInstance _wallinstances (Math|Transform|MakeTransform (Math|Vector|MakeVector (select (== _index (Class|KismetSystemLibrary|MakeLiteralInteger)) (- (+ (* (Math|Conversions|ToFloat(Integer) _index_2) (Math|Float|MakeLiteralFloat 5e+03)) (Math|Float|MakeLiteralFloat 2.5e+03)) (Math|Float|MakeLiteralFloat 3e+04)) (select (== _index (Class|KismetSystemLibrary|MakeLiteralInteger 1)) (Math|Float|MakeLiteralFloat 3e+04) (select (== _index (Class|KismetSystemLibrary|MakeLiteralInteger 2)) (- (Math|Float|MakeLiteralFloat 0.0) (- (+ (* (Math|Conversions|ToFloat(Integer) _index_2) (Math|Float|MakeLiteralFloat 5e+03)) (Math|Float|MakeLiteralFloat 2.5e+03)) (Math|Float|MakeLiteralFloat 3e+04))) (Math|Float|MakeLiteralFloat -3e+04)))) (select (== _index (Class|KismetSystemLibrary|MakeLiteralInteger)) (Math|Float|MakeLiteralFloat -3e+04) (select (== _index (Class|KismetSystemLibrary|MakeLiteralInteger 1)) (- (+ (* (Math|Conversions|ToFloat(Integer) _index_2) (Math|Float|MakeLiteralFloat 5e+03)) (Math|Float|MakeLiteralFloat 2.5e+03)) (Math|Float|MakeLiteralFloat 3e+04)) (select (== _index (Class|KismetSystemLibrary|MakeLiteralInteger 2)) (Math|Float|MakeLiteralFloat 3e+04) (- (Math|Float|MakeLiteralFloat 0.0) (- (+ (* (Math|Conversions|ToFloat(Integer) _index_2) (Math|Float|MakeLiteralFloat 5e+03)) (Math|Float|MakeLiteralFloat 2.5e+03)) (Math|Float|MakeLiteralFloat 3e+04)))))) (select (== (Math|Integer|%(Integer) (+ (* _index (Class|KismetSystemLibrary|MakeLiteralInteger 12)) _index_2) 7) (Class|KismetSystemLibrary|MakeLiteralInteger 2)) (Math|Float|MakeLiteralFloat 5e+02) (Math|Float|MakeLiteralFloat 1e+03))) (Math|Rotator|MakeRotator 0.0 0.0 (* (Math|Conversions|ToFloat(Integer) _index) (Math|Float|MakeLiteralFloat 9e+01))) (select (== (Math|Integer|%(Integer) (+ (* _index (Class|KismetSystemLibrary|MakeLiteralInteger 12)) _index_2) 7) (Class|KismetSystemLibrary|MakeLiteralInteger 2)) (Math|Vector|MakeVector 3e+01 5.0 2e+01) (Math|Vector|MakeVector 5e+01 5.0 3e+01))) false)))))